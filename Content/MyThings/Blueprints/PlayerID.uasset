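; PlayerID is a Blueprint that labels a player by passing a number and colour to a PlayerCard shown through its widget component.
; On BeginPlay it casts the component's widget to PlayerCard and copies its Num and Col variables into the card's PlayerNum and PlayerColour.
; Tick is disabled, and a duplicate of the assignment logic in the construction script graph is left unconnected.
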(event `self.ReceiveBeginPlay`
  (bind _asplayer_card (cast `/Game/MyThings/Widgets/PlayerCard` (`WidgetComponent.GetWidget` (`self.Widget`))))
  (set `/Game/MyThings/Widgets/PlayerCard.Player Num` (`self.Num`) _asplayer_card)
  (set `/Game/MyThings/Widgets/PlayerCard.Player Colour` (`self.Col`) _asplayer_card))

(fn `UserConstructionScript`)